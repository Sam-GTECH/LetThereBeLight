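; Test actor that moves vertically in step with the day cycle, apparently a stand-in for a material-driven effect.
; It stores its starting Z on BeginPlay.
; Each Tick it looks up the BP_DayCycleController_Plate actor and lerps its height from that Z to an OffsetZ above it by CycleAlpha, keeping X and Y.
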(event `self.ReceiveBeginPlay`
  (bind (_returnvalue_x _returnvalue_y _returnvalue_z) (`KismetMathLibrary.BreakVector` (`self.K2_GetActorLocation`)))
  (set `self.DefaultZ` _returnvalue_z))

(event `self.ReceiveTick`
  (params (DeltaSeconds :type "Float (single-precision)"))
  (bind (_returnvalue_x _returnvalue_y) (`KismetMathLibrary.BreakVector` (`self.K2_GetActorLocation`)))
  (bind _returnvalue (`GameplayStatics.GetActorOfClass` "/Game/Blueprint/BP_DayCycleController_Plate.BP_DayCycleController_Plate_C"))
  (`self.K2_SetActorLocation` (`KismetMathLibrary.MakeVector` _returnvalue_x _returnvalue_y (`KismetMathLibrary.Lerp` (`self.DefaultZ`) (+ (`self.DefaultZ`) (`self.OffsetZ`)) (`/Game/Blueprint/BP_DayCycleController.CycleAlpha` _returnvalue)))))

(fn `UserConstructionScript`)