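; Day/night controller that toggles the scene between day and night through SwitchDayNight, which plays or reverses DayNightTimeline.
; BeginPlay caches the starting intensity of every light in the DayLights and NightLights sets.
; The timeline's alpha lerps the directional light's pitch between night and day rotations.
; UpdateLightIntensityOfSet scales cached intensities by that alpha, inverted for night lights, so the two sets cross-fade.
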(event `self.ReceiveBeginPlay`
  (bind _result (`BlueprintSetLibrary.Set_Union` (`self.DayLights`) (`self.NightLights`)))
  (bind _valuepin (`|SetForEach` _result)
    (:`then`
      (`BlueprintMapLibrary.Map_Add` (`self.LightsBaseIntensity`) _valuepin (`LightComponentBase.Intensity` (`Light.LightComponent` _valuepin))))))

(event `self.ReceiveTick`
  (params (DeltaSeconds :type "Float (single-precision)")))

(fn `SwitchDayNight`
  (bind _daynighttimeline (`self.DayNightTimeline`))
  (`KismetSystemLibrary.PrintString` "Switch Day/Night")
  (bind _output_get (set `self.isDay` (not (`self.isDay`))))
  (if _output_get
    (`TimelineComponent.Play` _daynighttimeline)
    (else
      (`TimelineComponent.Reverse` _daynighttimeline))))

(fn `UpdateLightIntensityOfSet`
  (params (Lights :type "Set of Light Object Reference") (Alpha :type "Float (double-precision)") (Reverse :type Boolean))
  (locals (LocalAlpha :type "Float (double-precision)"))
  (if Reverse
    (set `local.LocalAlpha` (- 1.0 Alpha))
    (else
      (set `local.LocalAlpha` Alpha)))
  (bind _valuepin (`|SetForEach` Lights)
    (:`then`
      (`LightComponent.SetIntensity` (`Light.LightComponent` _valuepin) (* (`BlueprintMapLibrary.Map_Find` (`self.LightsBaseIntensity`) _valuepin) (`local.LocalAlpha`))))))

(fn `UserConstructionScript`)